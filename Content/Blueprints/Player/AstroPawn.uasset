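; Astronaut pawn for a calibrated perturbed-motion experiment, with physics-driven side thrusters and phase-driven back thruster effects.
; Calibration chains BP_Mover probes through origin adjustment, reachable-zone search and perturbed motion using CSV perturbations, saving results to ExperimentSaveGame.
; Testing has QTComponent find a saddle point in the saved points, then runs ExperimentExecution on the simulated body.
; On completion the body freezes and QTComponent's position-based score goes to the UI widget.
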(event `StartCalibration`
  (`KismetArrayLibrary.Array_Clear` (`/Game/Blueprints/GameSettings/ExperimentSaveGame.PerturbationPoints` (`self.Save Game`)))
  (`self.K2_SetActorLocationAndRotation` (-100.0 0.0 0.0))
  (`self.SendProbe` "AdjustOrigin"))

(event `self.ReceiveBeginPlay`
  (bind _configname (`self.ConfigName`))
  ;[1 1 1] Begin Play
  (if (`HeadMountedDisplayFunctionLibrary.IsHeadMountedDisplayEnabled`)
    (`HeadMountedDisplayFunctionLibrary.SetTrackingOrigin` "Eye"))
  (bind _returnvalue (`GameplayStatics.DoesSaveGameExist` _configname))
  (if _returnvalue
    (bind _returnvalue_2 (`GameplayStatics.LoadGameFromSlot` _configname))
    (bind _asexperiment_save_game (cast `/Game/Blueprints/GameSettings/ExperimentSaveGame` _returnvalue_2)
      (:`then`
        (set `self.Save Game` _asexperiment_save_game))
      (:`CastFailed`
        _))
    (else
      (bind _returnvalue_3 (`GameplayStatics.CreateSaveGameObject` "/Game/Blueprints/GameSettings/ExperimentSaveGame.ExperimentSaveGame_C"))
      (set `self.Save Game` _returnvalue_3)))
  (bind _asbp_gi (cast `/Game/Blueprints/GameSettings/BP_GI` (`GameplayStatics.GetGameInstance`)))
  (set `self.As BP GI` _asbp_gi))

(event `SendProbe`
  (params (TargetState :type "EExperimentState Enum" :default "WaitingForStart"))
  (bind (_returnvalue_location _returnvalue_rotation) (`KismetMathLibrary.BreakTransform` (`self.GetTransform`)))
  ;[1 1 1] Probe sending
  (`/Engine/EditorBlueprintResources/StandardMacros.IsValid` (`self.Probe`)
    (:`Is Not Valid`
      (switch `EExperimentState` TargetState
        (:`AdjustOrigin`
          (bind _returnvalue (`|SpawnActorFromClass` "/Game/Blueprints/Player/BP_Mover.BP_Mover_C" (`KismetMathLibrary.MakeTransform` (+ (* (`self.GetActorForwardVector`) 100.0) _returnvalue_location) _returnvalue_rotation) "Undefined" "OverrideRootScale" null (`self.Perturbations`) 2.0 TargetState null :!label _label))
          (bind _output_get (set `self.Probe` _returnvalue))
          (add `/Game/Blueprints/Player/BP_Mover.Finished` _output_get (`|CreateDelegate` :!event `OnProbeFinished`))
          (add `/Game/Blueprints/Player/BP_Mover.SinglePerturbationPointFound` _output_get (`|CreateDelegate` :!event `OnPerturbedMotion`)))
        (:`ReachableZoneSearch`
          (goto _label))
        (:`PerturbedMotion`
          (`self.PreparePerturbations`)
          (goto _label))
        (:`Finished`
          (`self.OnProbeFinished` TargetState))))))

(event `self.ReceiveTick`
  (params (DeltaSeconds :type "Float (single-precision)"))
  (bind _experimentexecution (`self.ExperimentExecution`))
  (bind _returnvalue (`ExperimentExecutionComponent.GetCurrentPhase` _experimentexecution))
  ;[1 1 1] Tick
  (if (and (`ActorComponent.IsActive` _experimentexecution) (or (`|EnumEquality` _returnvalue "Acceleration") (`|EnumEquality` _returnvalue "Decceleration")))
    (`ActorComponent.Activate` (`self.BackThruster`) false)
    (`ActorComponent.Activate` (`self.BackThruster1`) false)
    (else
      (`ActorComponent.Deactivate` (`self.BackThruster1`))
      (`ActorComponent.Deactivate` (`self.BackThruster`)))))

(event `OnProbeFinished`
  (params (InitialState :type "EExperimentState Enum" :default "WaitingForStart"))
  (bind _save_game (`self.Save Game`))
  ;[1 1 1] On probe finished
  (`self.StageFinished` InitialState)
  (switch `EExperimentState` InitialState
    (:`AdjustOrigin`
      (`self.OnAdjustOrigin`)
      (`self.CallDestroyOnProbe`)
      (`self.SendProbe` "ReachableZoneSearch"))
    (:`ReachableZoneSearch`
      (`self.OnMaxControl`)
      (`self.CallDestroyOnProbe`)
      (`self.SendProbe` "PerturbedMotion"))
    (:`PerturbedMotion`
      (`self.CallDestroyOnProbe`)
      (`self.SendProbe` "Finished"))
    (:`Finished`
      (set `/Game/Blueprints/GameSettings/ExperimentSaveGame.Perturbations` (`self.Perturbations`) _save_game)
      (`AsyncActionHandleSaveGame.AsyncSaveGameToSlot` self _save_game (`self.ConfigName`)))))

(event `MoveCameraHorizontal`
  (params (AxisScale :type "Float (double-precision)"))
  (bind _camerainput_x (`KismetMathLibrary.BreakVector2D` (`self.CameraInput`)))
  ;[1 1 1] Camera movement
  (set `self.CameraInput` (`KismetMathLibrary.MakeVector2D` _camerainput_x AxisScale)))

(event `ThrustRight`
  (params (AxisScale :type "Float (double-precision)"))
  ;[1 1 1] Astronaut controls
  (if (and (> AxisScale 0.0) (`SceneComponent.IsSimulatingPhysics` (`self.Cube1`) "None"))
    (`PrimitiveComponent.AddForce` (`self.Cube1`) (* (`SceneComponent.GetRightVector` (`self.Cube1`)) (* (`self.MaxThrust`) AxisScale)) "None" false)
    (`ActorComponent.Activate` (`self.LeftThruster`) false)
    (else
      (`ActorComponent.Deactivate` (`self.LeftThruster`)))))

(event `MoveCameraVertical`
  (params (AxisScale :type "Float (double-precision)"))
  (bind (_camerainput_x _camerainput_y) (`KismetMathLibrary.BreakVector2D` (`self.CameraInput`)))
  ;[1 1 1] Camera movement
  (set `self.CameraInput` (`KismetMathLibrary.MakeVector2D` AxisScale _camerainput_y)))

(event `ThrustLeft`
  (params (AxisScale :type "Float (double-precision)"))
  ;[1 1 1] Astronaut controls
  (if (and (`SceneComponent.IsSimulatingPhysics` (`self.Cube1`) "None") (< AxisScale 0.0))
    (`PrimitiveComponent.AddForce` (`self.Cube1`) (* (`SceneComponent.GetRightVector` (`self.Cube1`)) (* AxisScale (`self.MaxThrust`))) "None" false)
    (`ActorComponent.Activate` (`self.RightThruster`) false)
    (else
      (`ActorComponent.Deactivate` (`self.RightThruster`)))))

(event `OnAdjustOrigin`
  (bind _save_game (`self.Save Game`))
  ;[1 1 1] On adjust origin
  (bind _output_get (set `/Game/Blueprints/GameSettings/ExperimentSaveGame.InitialPosition` (`self.K2_GetActorLocation` (`self.Probe`)) _save_game))
  (set `/Game/Blueprints/GameSettings/ExperimentSaveGame.TargetPosition` (0.0 0.0 0.0) _save_game)
  (`self.K2_SetActorLocation` (+ (* (`self.GetActorForwardVector`) 100.0) _output_get) false true)
  (`self.K2_SetActorRotation` (struct :`Yaw` 180.0) true))

(event `SetIsZooming`
  (params (IsZooming :type Boolean))
  ;[1 1 1] Camera movement
  (set `self.IsZooming` IsZooming))

(event `OnMaxControl`
  (bind _returnvalue (`self.K2_GetActorLocation` (`self.Probe`)))
  (bind _reachablezonelimits (`/Game/Blueprints/GameSettings/ExperimentSaveGame.ReachableZoneLimits` (`self.Save Game`)))
  ;[1 1 1] On max control
  (`KismetArrayLibrary.Array_Set` _reachablezonelimits 1 _returnvalue)
  (`KismetArrayLibrary.Array_Set` _reachablezonelimits 0 (* _returnvalue -1.0)))

(event `OnPerturbedMotion`
  ;[1 1 1] On perturbed motion
  (`KismetArrayLibrary.Array_Add` (`/Game/Blueprints/GameSettings/ExperimentSaveGame.PerturbationPoints` (`self.Save Game`)) (`self.K2_GetActorLocation` (`self.Probe`))))

(event `CallDestroyOnProbe`
  ;[1 1 1] Probe destruction
  (bind _probe (`self.Probe`)
    (:`then`
      (`self.SetActorHiddenInGame` _probe false)
      (`self.K2_DestroyActor` _probe))
    (:`else`)))

(event `StartTesting`
  (bind _experimentexecution (`self.ExperimentExecution`))
  (bind _save_game (`self.Save Game`))
  (bind _reachablezonelimits (`/Game/Blueprints/GameSettings/ExperimentSaveGame.ReachableZoneLimits` _save_game))
  (bind _returnvalue (`GameplayStatics.DoesSaveGameExist` (`self.ConfigName`)))
  (if _returnvalue
    (`self.K2_SetActorLocationAndRotation` (`/Game/Blueprints/GameSettings/ExperimentSaveGame.InitialPosition` (`self.Save Game`)) (struct :`Yaw` 180.0) false true)
    (bind _returnvalue_2 (`QualityTestingComponent.FindSaddlePoint` (`self.QTComponent`) (`/Game/Blueprints/GameSettings/ExperimentSaveGame.PerturbationPoints` _save_game) (`|GetArrayItem` _reachablezonelimits) (`|GetArrayItem` _reachablezonelimits 1)))
    (bind _output_get (set `self.SaddlePointFound` _returnvalue_2))
    (if _output_get
      (`ActorComponent.SetActive` _experimentexecution true true)
      (`ExperimentExecutionComponent.SetupComponent` _experimentexecution (make `ExecutionComponentInitializer` false (`QualityTestingComponent.GetSaddlePointIdx` (`self.QTComponent`)) "PerturbedMotion" 0.0 20.0 400.0 2000.0 self (`/Game/Blueprints/GameSettings/ExperimentSaveGame.Perturbations` (`self.Save Game`))))
      (`PrimitiveComponent.SetSimulatePhysics` (`self.Cube1`) true)
      (else
        (`KismetSystemLibrary.PrintString` "NO SADDLE POINT")))))

(event `self.ExperimentExecution.OnComponentFinished`
  (bind _cube1 (`self.Cube1`))
  (`ActorComponent.SetComponentTickEnabled` (`self.ExperimentExecution`) false)
  (`PrimitiveComponent.SetPhysicsLinearVelocity` _cube1 (0.0 0.0 0.0) false "None")
  (`PrimitiveComponent.SetPhysicsAngularVelocityInRadians` _cube1 (0.0 0.0 0.0) false "None")
  (`PrimitiveComponent.SetSimulatePhysics` (`self.Cube1`) false)
  (`ActorComponent.SetActive` (`self.ExperimentExecution`) false true)
  (bind _asmain_user_widget (cast `/Game/Blueprints/UI/MainUserWidget` (`WidgetComponent.GetWidget` (`self.Widget`))))
  (`/Game/Blueprints/UI/MainUserWidget.SetScore` _asmain_user_widget (`QualityTestingComponent.EvaluateScore` (`self.QTComponent`) (`self.K2_GetActorLocation`))))

(event `self.ExperimentExecution.OnComponentUpdate`
  (params (CurrentTime :type "Float (single-precision)"))
  (`/Game/Blueprints/GameSettings/BP_GI.TimeUpdate` (`self.As BP GI`) CurrentTime))

(fn `GetInertiaTensor`
  (returns (ReturnValue :type "Vector Structure"))
  (return (38.799999 12.5 39.400002)))

(fn `GetPhysicsBody`
  (returns (ReturnValue :type "PrimitiveComponent Object Reference"))
  (return (`self.Cube1`)))

(fn `UserConstructionScript`)