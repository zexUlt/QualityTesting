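; BP_Mover is a probe actor that runs an experiment in calibration mode toward a target state with configured perturbations.
; After a start delay it initializes its ExperimentExecution component, supplying the probe mesh as physics body and a hard-coded inertia tensor through getters.
; It relays time updates to BP_GI and broadcasts perturbation completions.
; Completion plays a Niagara pulse whose end broadcasts Finished, while setup failure destroys the actor.
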(event `ActivateComponent`
  (bind _experimentexecution (`self.ExperimentExecution`))
  (`ActorComponent.Activate` _experimentexecution false)
  (`ExperimentExecutionComponent.SetupComponent` _experimentexecution (make `ExecutionComponentInitializer` true 0 (`self.TargetState`) 0.0 20.0 400.0 2000.0 self (`self.Perturbations`))))

(event `self.ReceiveBeginPlay`
  (`KismetSystemLibrary.K2_SetTimerDelegate` (delegate `ActivateComponent`) (`self.StartDelay`))
  (bind _asbp_gi (cast `/Game/Blueprints/GameSettings/BP_GI` (`GameplayStatics.GetGameInstance`)))
  (set `self.As BP GI` _asbp_gi))

(event `self.NS_Pulse.OnSystemFinished`
  (params (PSystem :type "NiagaraComponent Object Reference"))
  (`self.Finished` (`self.TargetState`)))

(event `self.ExperimentExecution.OnSinglePerturbationComplete`
  (`self.SinglePerturbationPointFound`))

(event `self.ExperimentExecution.OnComponentFinished`
  (`ActorComponent.Activate` (`self.NS_Pulse`) false))

(event `self.ExperimentExecution.OnComponentUpdate`
  (params (CurrentTime :type "Float (single-precision)"))
  (`/Game/Blueprints/GameSettings/BP_GI.TimeUpdate` (`self.As BP GI`) CurrentTime))

(event `self.ExperimentExecution.OnSetupFailed`
  (`KismetSystemLibrary.PrintString` "Fail")
  (`self.K2_DestroyActor`))

(fn `GetInertiaTensor`
  (returns (ReturnValue :type "Vector Structure"))
  (return (38.799999 12.5 39.400002)))

(fn `GetPhysicsBody`
  (returns (ReturnValue :type "PrimitiveComponent Object Reference"))
  (return (`self.ProbeMesh`)))

(fn `UserConstructionScript`)