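; Player controller that turns input into commands for the possessed AstroPawn: camera, thrust, zoom, probes, calibration and testing.
; On possess it binds the pawn's StageFinished event and rebroadcasts it as StagePassed.
; The HUD supplies the experiment stage for probe launches and the widget focused when ShowMenu toggles cursor and input mode.
; The HUD lookup and initial game-only input setup are disconnected, leaving BeginPlay empty.
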(event `self.ReceiveBeginPlay`)

(event `StageFinished_Event_0`
  (params (Stage :type "EExperimentState Enum" :default "WaitingForStart"))
  (`self.StagePassed` Stage))

(event `self.ReceivePossess`
  (params (PossessedPawn :type "Pawn Object Reference"))
  (bind _asastro_pawn (cast `/Game/Blueprints/Player/AstroPawn` PossessedPawn))
  (bind _output_get (set `self.AstroPawn` _asastro_pawn))
  (add `/Game/Blueprints/Player/AstroPawn.StageFinished` _output_get (delegate `StageFinished_Event_0`)))

(event `InputAxis|MoveCameraUp`
  (params (AxisValue :type "Float (single-precision)"))
  ;[1 1 1] Axis Mappings
  (`/Game/Blueprints/Player/AstroPawn.MoveCameraVertical` (`self.AstroPawn`) AxisValue))

(event `InputAction|SendProbe`
  (params (Key :type "Key Structure"))
  ;[1 1 1] Action Mappings
  (:`Pressed`
    (`/Game/Blueprints/Player/AstroPawn.SendProbe` (`self.AstroPawn`) (`/Game/Blueprints/GameSettings/BP_HUD.GetSelectedExperimentStage` (`self.HUD`)))))

(event `InputAxis|MoveCameraRight`
  (params (AxisValue :type "Float (single-precision)"))
  ;[1 1 1] Axis Mappings
  (`/Game/Blueprints/Player/AstroPawn.MoveCameraHorizontal` (`self.AstroPawn`) AxisValue))

(event `InputAxis|ThrustRight`
  (params (AxisValue :type "Float (single-precision)"))
  (bind _astropawn (`self.AstroPawn`))
  ;[1 1 1] Axis Mappings
  (`/Game/Blueprints/Player/AstroPawn.ThrustRight` _astropawn AxisValue)
  (`/Game/Blueprints/Player/AstroPawn.ThrustLeft` _astropawn AxisValue))

(event `InputAction|ShowMenu`
  (params (Key :type "Key Structure"))
  ;[1 1 1] Action Mappings
  (:`Pressed`
    (`/Engine/EditorBlueprintResources/StandardMacros.FlipFlop`
      (:`A`
        (`WidgetBlueprintLibrary.SetInputMode_GameAndUIEx` self (`/Game/Blueprints/GameSettings/BP_HUD.MainWidget` (`self.HUD`)))
        (set `self.bShowMouseCursor` true))
      (:`B`
        (`WidgetBlueprintLibrary.SetInputMode_GameOnly` self)
        (set `self.bShowMouseCursor` false)))))

(event `InputAction|DestroyProbe`
  (params (Key :type "Key Structure"))
  ;[1 1 1] Action Mappings
  (:`Pressed`
    (`/Game/Blueprints/Player/AstroPawn.CallDestroyOnProbe` (`self.AstroPawn`))))

(event `InputAction|StartTesting`
  (params (Key :type "Key Structure"))
  ;[1 1 1] Action Mappings
  (:`Pressed`
    (`/Game/Blueprints/Player/AstroPawn.StartTesting` (`self.AstroPawn`))))

(event `InputAction|Zoom`
  (params (Key :type "Key Structure"))
  (bind _astropawn (`self.AstroPawn`))
  ;[1 1 1] Action Mappings
  (:`Pressed`
    (`/Game/Blueprints/Player/AstroPawn.SetIsZooming` _astropawn true))
  (:`Released`
    (`/Game/Blueprints/Player/AstroPawn.SetIsZooming` _astropawn false)))

(event `InputAction|StartCalibration`
  (params (Key :type "Key Structure"))
  ;[1 1 1] Action Mappings
  (:`Pressed`
    (`/Game/Blueprints/Player/AstroPawn.StartCalibration` (`self.AstroPawn`))))

(fn `UserConstructionScript`)