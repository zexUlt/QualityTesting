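; Earth environment Blueprint that continuously spins its Earth component around that component's up vector.
; On BeginPlay, a math expression derives a constant angular velocity as two pi divided by a fixed period.
; Each Tick scales that velocity by delta time and applies it as an axis-angle world rotation, keeping the spin frame-rate independent.
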(event EventTick
  (params (DeltaSeconds :type Float%20%28single-precision%29))
  (Transformation|AddWorldRotation (Variables|Default|GetEarth) (Math|Vector|RotatorfromAxisandAngle (Math|Vector|GetUpVector (Variables|Default|GetEarth)) (* (Variables|Default|GetAngularVelocity) DeltaSeconds)) false false))

(event EventBeginPlay
  (Variables|Default|SetAngularVelocity (|((2*Pi)/8.634400) 3.141593)))

(fn ConstructionScript)